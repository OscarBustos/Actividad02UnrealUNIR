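; BP_EnemyProjectile is a timed grenade projectile whose explosion spares actors tagged "Enemy".
; On BeginPlay it waits out a fuse delay, then spawns explosion particles and sound at the mesh location.
; It applies full radial damage with no falloff, passing all "Enemy"-tagged actors as the ignore list, then destroys itself.
; Mesh hits only play a bounce sound, so impact does not trigger detonation.
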(event OnComponentHit(StaticMesh)
  (params (HitComponent :type Primitive%20Component%20Object%20Reference) (OtherActor :type Actor%20Object%20Reference) (OtherComp :type Primitive%20Component%20Object%20Reference) (NormalImpulse :type Vector :default "0, 0, 0") (Hit :type Hit%20Result%20Structure%20%28by%20ref%29))
  (Audio|PlaySoundatLocation "/Game/00Project/Guns/GrenadeLauncher/MilitaryWeapDark/Sound/GrenadeLauncher/GrenadeLauncher_Bounce_Cue.GrenadeLauncher_Bounce_Cue" (Transformation|GetWorldLocation (Variables|Default|GetStaticMesh)) "0, 0, 0" 0.15 1.0 0.0 "/Game/00Project/Guns/GrenadeLauncher/MilitaryWeapDark/Sound/Attenuation/ProjectileImpact_att.ProjectileImpact_att" 0 0 0))

(event EventBeginPlay
  (bind _staticmesh (Variables|Default|GetStaticMesh))
  (bind _returnvalue (Transformation|GetWorldLocation _staticmesh))
  (Utilities|FlowControl|Delay (Variables|Default|GetExplosionDelay))
  (Effects|SpawnEmitteratLocation "/Game/00Project/Guns/GrenadeLauncher/MilitaryWeapDark/FX/P_Grenade_Explosion_01.P_Grenade_Explosion_01" _returnvalue)
  (Audio|PlaySoundatLocation "/Game/00Project/Guns/GrenadeLauncher/MilitaryWeapDark/Sound/GrenadeLauncher/GrenadeLauncher_Explosion_Cue.GrenadeLauncher_Explosion_Cue" _returnvalue "0, 0, 0" 1.0 1.0 0.0 "/Game/00Project/Guns/GrenadeLauncher/MilitaryWeapDark/Sound/Attenuation/Explosion_att.Explosion_att" 0 0 0)
  (bind _outactors (Actor|GetAllActorswithTag "Enemy"))
  (Game|Damage|ApplyRadialDamage (Variables|Default|GetDamage) _returnvalue (Variables|Default|GetDamage%20Radius) 0 _outactors self 0 true "ECC_Visibility")
  (Actor|DestroyActor))

(fn ConstructionScript)