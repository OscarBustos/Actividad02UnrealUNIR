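; BP_Win is a level-goal actor that lets the player win on entering its WinnerTrigger with enough score.
; On overlap by BP_AmyCharacter, it compares the game instance's Score against RequiredCoins.
; If met, it shows WBP_WinMenu with the mouse cursor and game-and-UI input, then pauses the game.
; Otherwise it plays an error sound at the actor's location.
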(event OnComponentBeginOverlap(WinnerTrigger)
  (params (OverlappedComponent :type Primitive%20Component%20Object%20Reference) (OtherActor :type Actor%20Object%20Reference) (OtherComp :type Primitive%20Component%20Object%20Reference) (OtherBodyIndex :type Integer) (bFromSweep :type Boolean) (SweepResult :type Hit%20Result%20Structure%20%28by%20ref%29))
  (bind _returnvalue (Game|GetPlayerController 0))
  (bind _asbp_amy_character (Utilities|Casting|CastToBP_AmyCharacter OtherActor))
  (if (>= (Variables|/Game/00Project/Blueprints/BP_GameInstance.BP_GameInstance_C|GetScore (Variables|/Game/00Project/Characters/Amy/Blueprints/BP_AmyCharacter.BP_AmyCharacter_C|GetAs%20BP%20Game%20Instance _asbp_amy_character)) (Variables|Default|GetRequiredCoins))
    (bind _returnvalue_2 (UserInterface|CreateWidget "/Game/00Project/UI/Blueprints/WBP_WinMenu.WBP_WinMenu_C" _returnvalue))
    (UserInterface|Viewport|AddtoViewport _returnvalue_2 0)
    (Input|SetInputModeGameandUI _returnvalue _returnvalue_2 "DoNotLock" true false)
    (Variables|/Script/Engine.PlayerController|SetbShowMouseCursor _returnvalue true)
    (Game|SetGamePaused true)
    (else
      (Audio|PlaySoundatLocation "/Game/00Project/UI/Audio/error_003.error_003" (Transformation|GetActorLocation) "0, 0, 0" 1.0 1.0 0.0 0 0 0 0))))

(event EventBeginPlay)

(event Collision|EventActorBeginOverlap
  (params (OtherActor :type Actor%20Object%20Reference)))

(event EventTick
  (params (DeltaSeconds :type Float%20%28single-precision%29)))

(fn ConstructionScript)