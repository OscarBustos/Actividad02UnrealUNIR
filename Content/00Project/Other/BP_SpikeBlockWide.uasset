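; BP_SpikeBlockWide is a spike block hazard that applies damage to pawns touching its Box.
; Begin overlap damages the pawn immediately and sets an overlap flag, which end overlap clears for any actor.
; While the flag is set, Tick restarts a Retriggerable Delay each frame, so its follow-up hit on the last cast pawn lands DamageDelay after those restarts stop, rather than repeating during contact.
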(event OnComponentBeginOverlap(Box)
  (params (OverlappedComponent :type Primitive%20Component%20Object%20Reference) (OtherActor :type Actor%20Object%20Reference) (OtherComp :type Primitive%20Component%20Object%20Reference) (OtherBodyIndex :type Integer) (bFromSweep :type Boolean) (SweepResult :type Hit%20Result%20Structure%20%28by%20ref%29))
  (bind _aspawn (Utilities|Casting|CastToPawn OtherActor))
  (CallFunction|DamagePawn _aspawn)
  (Variables|Default|SetIsPawnOverlapping true))

(event OnComponentEndOverlap(Box)
  (params (OverlappedComponent :type Primitive%20Component%20Object%20Reference) (OtherActor :type Actor%20Object%20Reference) (OtherComp :type Primitive%20Component%20Object%20Reference) (OtherBodyIndex :type Integer))
  (Variables|Default|SetIsPawnOverlapping false))

(event Custom|DamagePawn
  (params (Pawn :type Pawn%20Object%20Reference))
  (Utilities|IsValid Pawn
    (:Is%20Valid
      (Game|Damage|ApplyDamage Pawn (Variables|Default|GetDamage) 0 self))))

(event EventTick
  (params (DeltaSeconds :type Float%20%28single-precision%29))
  (if (Variables|Default|GetIsPawnOverlapping)
    (Utilities|FlowControl|RetriggerableDelay (Variables|Default|GetDamageDelay))
    (CallFunction|DamagePawn (stale OnComponentBeginOverlap(Box) _aspawn))))

(fn ConstructionScript)