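; Slime character that patrols between two points, damages whatever it hits and can be killed.
; Path points detach at BeginPlay; Tick drives movement toward the target, with FlipFlops swapping target and facing on arrival.
; Damage lowers health and sets hit flags, with WasHit clearing on a timer; death stops movement and destroys it after a delay.
; Overlap begin and end with Player-tagged actors toggle CanAttack.
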(event Custom|SetPatrolPoint
  ;[1 1 1] Patrol
  (Utilities|FlowControl|FlipFlop
    (:A
      (Variables|Default|SetTargetPatrolPoint (Transformation|GetWorldLocation (Variables|Default|GetInitialPoint))))
    (:B
      (Variables|Default|SetTargetPatrolPoint (Transformation|GetWorldLocation (Variables|Default|GetFinalPoint))))))

(event Custom|ChangeRotation
  ;[1 1 1] Define rotation when direction changed
  (Utilities|FlowControl|FlipFlop
    (:A
      (Variables|Default|SetRotationDegrees 180))
    (:B
      (Variables|Default|SetRotationDegrees 0))))

(event EventBeginPlay
  (Transformation|DetachFromComponent (Variables|Default|GetPathPoints) "KeepWorld" "KeepWorld" "KeepWorld" true)
  (CallFunction|SetPatrolPoint))

(event Collision|EventActorBeginOverlap
  (params (OtherActor :type Actor%20Object%20Reference))
  (CallFunction|CalculateCanAttack OtherActor))

(event EventTick
  (params (DeltaSeconds :type Float%20%28single-precision%29))
  (bind _returnvalue (Transformation|GetActorLocation))
  (bind _targetpatrolpoint (Variables|Default|GetTargetPatrolPoint))
  (Utilities|FlowControl|Sequence
    (:then_0
      ;[1 1 1] Calculate direction and move
      (if (not (Variables|Default|GetIsDead))
        (Pawn|Input|AddMovementInput (Math|Vector|GetUnitDirection(Vector) _returnvalue _targetpatrolpoint) 0.5 false)
        (if (< (Math|Vector|Distance(Vector) _returnvalue _targetpatrolpoint) 1e+02)
          (CallFunction|SetPatrolPoint)
          (CallFunction|ChangeRotation)
          (Transformation|SetActorRotation (Math|Rotator|MakeRotator 0.0 0.0 (Math|Conversions|ToFloat(Integer) (Variables|Default|GetRotationDegrees)))))))
    (:then_1
      (if (Variables|Default|GetIsDead)
        (Utilities|FlowControl|Delay 2.0)
        (Actor|DestroyActor)))
    (:then_2
      (if (Variables|Default|GetWasHit)
        (Variables|Default|SetCurrentTimeHit (+ DeltaSeconds (Variables|Default|GetCurrentTimeHit)))
        (if (>= (Variables|Default|GetCurrentTimeHit) (Variables|Default|GetTimeBetweenHurt))
          (Variables|Default|SetWasHit false)
          (Variables|Default|SetCurrentTimeHit 0.0))))))

(event Collision|EventActorEndOverlap
  (params (OtherActor :type Actor%20Object%20Reference))
  (CallFunction|CalculateCanAttack OtherActor))

(event Game|Damage|EventAnyDamage
  (params (Damage :type Float%20%28single-precision%29) (DamageType :type Damage%20Type%20Object%20Reference) (InstigatedBy :type Controller%20Object%20Reference) (DamageCauser :type Actor%20Object%20Reference))
  (CallFunction|CalculateHealth 0 Damage)
  (Variables|Default|SetWasHit true)
  (Variables|Default|SetPlayHitAnimation true))

(event Collision|EventHit
  (params (MyComp :type Primitive%20Component%20Object%20Reference) (Other :type Actor%20Object%20Reference) (OtherComp :type Primitive%20Component%20Object%20Reference) (bSelfMoved :type Boolean) (HitLocation :type Vector :default "0, 0, 0") (HitNormal :type Vector :default "0, 0, 0") (NormalImpulse :type Vector :default "0, 0, 0") (Hit :type Hit%20Result%20Structure%20%28by%20ref%29))
  (Game|Damage|ApplyDamage Other (Variables|Default|GetDamage) 0 0))

(fn ConstructionScript)

(fn CalculateCanAttack
  (params (Actor :type Actor%20Object%20Reference))
  (if (Utilities|Array|ContainsItem (Variables|/Script/Engine.Actor|GetTags Actor) "Player")
    (Variables|Default|SetCanAttack (not (Variables|Default|GetCanAttack)))))

(fn CalculateHealth
  (params (Actor :type Actor%20Object%20Reference) (Damage :type Float%20%28double-precision%29))
  (bind _output_get (Variables|Default|SetHealth (- (Variables|Default|GetHealth) Damage)))
  (if (<= _output_get 0)
    (Variables|Default|SetIsDead true)))