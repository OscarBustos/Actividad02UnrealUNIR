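; BP_Timy_TO is a player-controlled Timy pawn that handles Enhanced Input movement.
; On BeginPlay it casts and stores its BP_TimyController, then adds the IMC_PlayerInput mapping context to that player's input subsystem.
; IA_Movement feeds AddMovementInput along vectors derived from control rotation: X strafes on the right vector (yaw and roll), Y moves on the yaw-only forward vector, ignoring camera pitch.
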(event Input|EnhancedActionEvents|EnhancedInputActionIA_Movement
  (params (ActionValue :type Vector%202D%20Structure) (ElapsedSeconds :type Float%20%28double-precision%29) (TriggeredSeconds :type Float%20%28double-precision%29) (InputAction :type Input%20Action%20Object%20Reference :default "/Game/00Project/Characters/Timy/Blueprints/IA_Movement.IA_Movement"))
  (bind _returnvalue (Pawn|GetControlRotation :!class /Script/Engine.Pawn))
  ;[1 1 1] Move
  (Pawn|Input|AddMovementInput (Math|Vector|GetRightVector (Math|Rotator|MakeRotator (.roll _returnvalue) 0.0 (.yaw _returnvalue))) (.x ActionValue) false)
  (Pawn|Input|AddMovementInput (Math|Vector|GetForwardVector (Math|Rotator|MakeRotator 0.0 0.0 (.yaw (Pawn|GetControlRotation :!class /Script/Engine.Pawn)))) (.y ActionValue) false))

(event EventBeginPlay
  (bind _asbp_timy_controller (Utilities|Casting|CastToBP_TimyController (Pawn|GetController)))
  (bind _output_get (Variables|Default|SetBPTimyController _asbp_timy_controller))
  (Utilities|IsValid (PlayerController|LocalPlayerSubsystems|GetEnhancedInputLocalPlayerSubsystem _output_get)
    (:Is%20Valid
      (Input|AddMappingContext (PlayerController|LocalPlayerSubsystems|GetEnhancedInputLocalPlayerSubsystem _output_get) "/Game/00Project/Characters/Timy/Blueprints/IMC_PlayerInput.IMC_PlayerInput" 0 "(bIgnoreAllPressedKeysUntilRelease=True,bForceImmediately=False,bNotifyUserSettings=False)"))))

(event Collision|EventActorBeginOverlap
  (params (OtherActor :type Actor%20Object%20Reference)))

(event EventTick
  (params (DeltaSeconds :type Float%20%28single-precision%29)))

(fn ConstructionScript)