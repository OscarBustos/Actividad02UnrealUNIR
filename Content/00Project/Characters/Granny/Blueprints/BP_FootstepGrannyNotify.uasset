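; BP_FootstepGrannyNotify is an animation notify that plays surface-dependent footstep sounds for the Granny character.
; On notify, it line-traces 200 units down from the owning actor along its up vector on the Visibility channel.
; The hit's physical surface type selects a grass or wood sound, played at the actor's location rather than at the foot.
; Only those two surfaces have sounds, and the trace's success is not checked.
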(fn ReceivedNotify
  (params (MeshComp :type Skeletal%20Mesh%20Component%20Object%20Reference) (Animation :type Anim%20Sequence%20Base%20Object%20Reference) (EventReference :type Anim%20Notify%20Event%20Reference%20Structure%20%28by%20ref%29))
  (bind _returnvalue (Components|GetOwner MeshComp))
  (bind _returnvalue_2 (Transformation|GetActorLocation _returnvalue))
  (bind _outhit (Collision|LineTraceByChannel _returnvalue_2 (+ _returnvalue_2 (* (Transformation|GetActorUpVector _returnvalue) -2e+02)) "TraceTypeQuery1" false 0 "None"))
  (if true
    (switch Utilities|FlowControl|Switch|SwitchonEPhysicalSurface (Collision|GetSurfaceType _outhit)
      (:SurfaceType1
        (Audio|PlaySoundatLocation "/Game/00Project/Characters/Amy/Audio/footstep_grass.footstep_grass" _returnvalue_2 "0, 0, 0" 0.67 1.0 0.0 "/Game/00Project/Guns/GrenadeLauncher/MilitaryWeapDark/Sound/Attenuation/WeaponShot_att.WeaponShot_att" 0 0 0))
      (:SurfaceType2
        (Audio|PlaySoundatLocation "/Game/00Project/Characters/Granny/Audio/footstep-wood-3.footstep-wood-3" _returnvalue_2 "0, 0, 0" 0.67 1.0 0.0 "/Game/00Project/Guns/GrenadeLauncher/MilitaryWeapDark/Sound/Attenuation/WeaponShot_att.WeaponShot_att" 0 0 0)))
    (return false)))