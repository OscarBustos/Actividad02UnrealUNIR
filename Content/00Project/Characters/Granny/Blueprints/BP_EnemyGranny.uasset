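; Granny enemy character that patrols between two points and shoots projectiles at the player on detection.
; Tick either walks toward the current patrol point, alternated by a FlipFlop with a wait, or turns toward the player and fires on a cooldown after a dot-product facing check.
; Detector overlaps switch between patrol and attack, and the game mode's player-death event restores patrol.
; Damage plays hit reactions until death, then destroys the actor after a delay.
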(event OnComponentBeginOverlap(Detector)
  (params (OverlappedComponent :type Primitive%20Component%20Object%20Reference) (OtherActor :type Actor%20Object%20Reference) (OtherComp :type Primitive%20Component%20Object%20Reference) (OtherBodyIndex :type Integer) (bFromSweep :type Boolean) (SweepResult :type Hit%20Result%20Structure%20%28by%20ref%29))
  ;[1 0.9321 0.3896] Player Detection Logic
  (if (not (Variables|/Game/ThirdPerson/Blueprints/TestMarc/BP_GameModeTest.BP_GameModeTest_C|GetIsPlayerDead? (Variables|Default|Getm_GameMode)))
    (bind _asbp_character_test (Utilities|Casting|CastToBP_CharacterTest OtherActor))
    (Utilities|IsValid _asbp_character_test
      (:Is%20Valid
        (Variables|Default|SetIsSeeingPlayer true)
        (Development|PrintString "HA DETECTADO" false)
        (Variables|Default|SetIsPatroling false)
        (Variables|Default|SetCanAttack? true)))))

(event OnComponentEndOverlap(Detector)
  (params (OverlappedComponent :type Primitive%20Component%20Object%20Reference) (OtherActor :type Actor%20Object%20Reference) (OtherComp :type Primitive%20Component%20Object%20Reference) (OtherBodyIndex :type Integer))
  ;[1 0.9321 0.3896] Player Detection Logic
  (if (not (Variables|/Game/ThirdPerson/Blueprints/TestMarc/BP_GameModeTest.BP_GameModeTest_C|GetIsPlayerDead? (Variables|Default|Getm_GameMode)))
    (Development|PrintString "YA NO DETECTA" false)
    (CallFunction|BacktoPatrol)))

(event Custom|Shoot
  (bind _spawnprojectilelocation (Variables|Default|GetSpawnProjectileLocation))
  (bind _returnvalue (Transformation|GetWorldLocation _spawnprojectilelocation))
  ;[1 0.4368 0.8] Shoot Logic
  (if (Variables|Default|GetCanAttack?)
    (Animation|PlayAnimMontage "/Game/00Project/Characters/Granny/Animations/FiringRifle_UE_Montage.FiringRifle_UE_Montage" 1.0 "None")
    (Game|SpawnActorfromClass "/Game/00Project/Guns/GrenadeLauncher/Blueprints/BP_EnemyProjectile.BP_EnemyProjectile_C" (Math|Transform|MakeTransform _returnvalue (Pawn|GetControlRotation :!class /Script/Engine.Pawn) "1.000000,1.000000,1.000000") "Undefined" "MultiplyWithRoot" 0 0)
    (Audio|PlaySoundatLocation "/Game/00Project/Guns/GrenadeLauncher/MilitaryWeapDark/Sound/GrenadeLauncher/GrenadeLauncherB_Fire_Cue.GrenadeLauncherB_Fire_Cue" _returnvalue "0, 0, 0" 0.25 1.0 0.0 "/Game/00Project/Guns/GrenadeLauncher/MilitaryWeapDark/Sound/Attenuation/WeaponShot_att.WeaponShot_att" 0 0 0)
    (Variables|Default|SetCanAttack? false)
    (Utilities|FlowControl|Delay (Variables|Default|GetShootDelay))
    (Variables|Default|SetCanAttack? true)))

(event Custom|RotateToActor
  (params (Actor :type Actor%20Object%20Reference))
  ;[0.5962 1 0.4873] Rotate Enemy to Actor
  (Utilities|IsValid Actor
    (:Is%20Valid
      (Transformation|SetActorRotation (Math|Rotator|MakeRotator 0.0 0.0 (.yaw (Math|Rotator|FindLookatRotation (Transformation|GetActorLocation) (Transformation|GetActorLocation Actor))))))))

(event Custom|Death
  (Variables|Default|SetIsPatroling false)
  (Variables|Default|SetIsSeeingPlayer false)
  (Variables|Default|SetCanAttack? false)
  (Variables|Default|SetIsDead true)
  (Utilities|FlowControl|Delay 2.9)
  (Actor|DestroyActor))

(event Custom|SetPatrolPoint
  (params (WaitTime :type Float%20%28double-precision%29))
  ;[1 0.9387 0.6514] Set Patrol Target
  (Utilities|FlowControl|DoOnce false :!label _label
    (:Completed
      (Utilities|FlowControl|Delay WaitTime)
      (Utilities|FlowControl|Sequence
        (:then_0
          (Utilities|FlowControl|FlipFlop
            (:A
              (Variables|Default|SetTargetPatrolPoint (Transformation|GetWorldLocation (Variables|Default|GetPatrolPoint1))))
            (:B
              (Variables|Default|SetTargetPatrolPoint (Transformation|GetWorldLocation (Variables|Default|GetPatrolPoint2))))))
        (:then_1
          (goto _label Reset))))))

(event Custom|BackToPatrol
  (Variables|Default|SetIsSeeingPlayer false)
  (Variables|Default|SetCanAttack? false)
  (Variables|Default|SetIsPatroling true))

(event EventBeginPlay
  (bind _asbp_game_mode_test (Utilities|Casting|CastToBP_GameModeTest (Game|GetGameMode)))
  (Utilities|IsValid _asbp_game_mode_test
    (:Is%20Valid
      (bind _output_get (Variables|Default|Setm_GameMode _asbp_game_mode_test))
      (EventDispatchers|BindEventtoOnPlayerDeath _output_get (delegate Custom|BackToPatrol))
      (Transformation|DetachFromComponent (Variables|Default|GetPatrolPoint1) "KeepWorld" "KeepWorld" "KeepWorld" true)
      (CallFunction|SetPatrolPoint 0.0))))

(event Game|Damage|EventAnyDamage
  (params (Damage :type Float%20%28single-precision%29) (DamageType :type Damage%20Type%20Object%20Reference) (InstigatedBy :type Controller%20Object%20Reference) (DamageCauser :type Actor%20Object%20Reference))
  (if (> (Variables|Default|GetHealth) 0.0)
    (Animation|PlayAnimMontage "/Game/00Project/Characters/Granny/Animations/HitReaction_UE_Montage.HitReaction_UE_Montage" 1.0 "None")
    (bind _output_get (Variables|Default|SetHealth (- (Variables|Default|GetHealth) Damage)))
    (if (<= _output_get 0.0)
      (CallFunction|Death)
      (Components|Animation|PlayAnimation (Variables|Character|GetMesh) "/Game/00Project/Characters/Granny/Animations/DeathFromTheFront_UE.DeathFromTheFront_UE" false))))

(event EventTick
  (params (DeltaSeconds :type Float%20%28single-precision%29))
  (if (not (Variables|Default|GetIsDead))
    (CallFunction|CheckFacingPlayer)
    ;[1 0.9387 0.6514] Patrol
    (if (Variables|Default|GetIsPatroling)
      (if (< (Math|Vector|Distance(Vector) (Transformation|GetActorLocation) (Variables|Default|GetTargetPatrolPoint)) 1e+02)
        (CallFunction|SetPatrolPoint 2.0)
        (else
          (Pawn|Input|AddMovementInput (Math|Vector|GetUnitDirection(Vector) (Transformation|GetActorLocation) (Variables|Default|GetTargetPatrolPoint)) (Variables|Default|GetSpeedMultiplier) false)))
      (else
        (CallFunction|RotatetoActor (Game|GetPlayerCharacter 0))
        (if (Variables|Default|GetIsFacingPlayer)
          (CallFunction|Shoot))))))

(fn ConstructionScript)

(fn CheckFacingPlayer
  (bind _m_gamemode (Variables|Default|Getm_GameMode))
  (bind _m_playercharacter (Variables|/Game/ThirdPerson/Blueprints/TestMarc/BP_GameModeTest.BP_GameModeTest_C|Getm_PlayerCharacter _m_gamemode))
  (Utilities|IsValid _m_playercharacter
    (:Is%20Valid
      (if (>= (Math|Vector|DotProduct (Transformation|GetActorForwardVector) (Math|Vector|GetUnitDirection(Vector) (Transformation|GetActorLocation) (Transformation|GetActorLocation _m_playercharacter))) 0.0)
        (Variables|Default|SetIsFacingPlayer true)
        (else
          (Variables|Default|SetIsFacingPlayer false :!label _label))))
    (:Is%20Not%20Valid
      (goto _label))))