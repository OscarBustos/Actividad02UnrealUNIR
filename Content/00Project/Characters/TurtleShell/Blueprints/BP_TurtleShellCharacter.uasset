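; Turtle shell enemy character that patrols between two points, tracks whether it can attack, and dies from bullet hits.
; On BeginPlay it detaches its path points, then Tick moves it toward the current target, with FlipFlops swapping target and yaw on arrival.
; Player-tagged overlaps toggle CanAttack on begin and end.
; Bullet-tagged overlaps reduce health, and at zero Tick destroys the actor after a short delay.
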(event Custom|SetPatrolPoint
  (Utilities|FlowControl|FlipFlop
    (:A
      (Variables|Default|SetTargetPatrolPoint (Transformation|GetWorldLocation (Variables|Default|GetInitialPoint))))
    (:B
      (Variables|Default|SetTargetPatrolPoint (Transformation|GetWorldLocation (Variables|Default|GetFinalPoint))))))

(event Custom|ChangeRotation
  (Utilities|FlowControl|FlipFlop
    (:A
      (Variables|Default|SetRotationDegrees 180))
    (:B
      (Variables|Default|SetRotationDegrees 0))))

(event EventBeginPlay
  (Transformation|DetachFromComponent (Variables|Default|GetPathPoints) "KeepWorld" "KeepWorld" "KeepWorld" true)
  (CallFunction|SetPatrolPoint))

(event Collision|EventActorBeginOverlap
  (params (OtherActor :type Actor%20Object%20Reference))
  (CallFunction|CalculateCanAttack OtherActor)
  (CallFunction|CalculateHealth OtherActor))

(event EventTick
  (params (DeltaSeconds :type Float%20%28single-precision%29))
  (bind _returnvalue (Transformation|GetActorLocation))
  (bind _targetpatrolpoint (Variables|Default|GetTargetPatrolPoint))
  (Utilities|FlowControl|Sequence
    (:then_0
      ;[1 1 1] Calculate direction and move
      (Pawn|Input|AddMovementInput (Math|Vector|GetUnitDirection(Vector) _returnvalue _targetpatrolpoint) 0.5 false)
      (if (< (Math|Vector|Distance(Vector) _returnvalue _targetpatrolpoint) 1e+02)
        (CallFunction|SetPatrolPoint)
        (CallFunction|ChangeRotation)
        (Transformation|SetActorRotation (Math|Rotator|MakeRotator 0.0 0.0 (Math|Conversions|ToFloat(Integer) (Variables|Default|GetRotationDegrees))))))
    (:then_1
      (if (Variables|Default|GetIsDead)
        (Utilities|FlowControl|Delay 0.2)
        (Actor|DestroyActor)))))

(event Collision|EventActorEndOverlap
  (params (OtherActor :type Actor%20Object%20Reference))
  (CallFunction|CalculateCanAttack OtherActor))

(fn ConstructionScript)

(fn CalculateCanAttack
  (params (Actor :type Actor%20Object%20Reference))
  (if (Utilities|Array|ContainsItem (Variables|/Script/Engine.Actor|GetTags Actor) "Player")
    (Variables|Default|SetCanAttack (not (Variables|Default|GetCanAttack)))))

(fn CalculateHealth
  (params (Actor :type Actor%20Object%20Reference))
  (if (Utilities|Array|ContainsItem (Variables|/Script/Engine.Actor|GetTags Actor) "Bullet")
    (bind _output_get (Variables|Default|SetHealth (- (Variables|Default|GetHealth) 1)))
    (if (<= _output_get 0)
      (Variables|Default|SetIsDead true))))